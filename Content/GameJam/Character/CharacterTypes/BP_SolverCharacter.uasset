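; BP_SolverCharacter is a playable character variant, named for a Solver role, that adds a crosshair and interaction input to its parent class.
; BeginPlay runs the parent logic, creates the WB_Crosshair widget, adds it to the viewport and prints a "Hello" debug string.
; Pressing and releasing E forwards the key state to the Interactor's InteractionInput under the default key.
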(event EventBeginPlay
  (|CallParentFunction)
  (bind _returnvalue (UserInterface|CreateWidget "/Game/GameJam/Widgets/Crosshair/WB_Crosshair.WB_Crosshair_C"))
  (UserInterface|Viewport|AddtoViewport _returnvalue 0)
  (Development|PrintString "Hello"))

(event Input|KeyboardEvents|E
  (params (Key :type Key%20Structure :default "None"))
  (:Pressed
    (Class|InteractorComponent|InteractionInput (Variables|Default|GetInteractor) "DefaultKey" true))
  (:Released
    (Class|InteractorComponent|InteractionInput (Variables|Default|GetInteractor) "DefaultKey" false)))

(fn ConstructionScript
  (|CallParentFunction))