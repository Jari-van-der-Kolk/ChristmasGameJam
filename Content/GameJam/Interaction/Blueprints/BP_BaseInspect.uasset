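; Base Blueprint for inspecting an item, showing its mesh alongside a UI with its name and description.
; Its Interaction event stores the character, sets the Item mesh, creates and displays WBP_Inspect, then calls DisableInput and EnableInput with the first player controller.
; The Interactable interface's OnInteract is only a placeholder that prints a debug string, and no logic here closes the inspection.
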(event OnInteract(Interactable)
  (params (Interactor :type Interactor%20Component%20Object%20Reference) (Interactable :type Interactable%20Component%20Object%20Reference))
  (Development|PrintString "Hello"))

(event EventInteraction
  (params (Charater :type BP%20Third%20Person%20Character%20Object%20Reference) (InspectedItem :type Static%20Mesh%20Object%20Reference) (ItemName :type Text) (ItemDescription :type Text))
  (bind _returnvalue (Game|GetPlayerController 0))
  (Variables|Default|SetCharater Charater)
  (Components|StaticMesh|SetStaticMesh (Variables|Default|GetItem) InspectedItem)
  (bind _returnvalue_2 (Game|ConstructObjectfromClass "/Game/GameJam/Interaction/Blueprints/WBP_Inspect.WBP_Inspect_C" ItemName ItemDescription))
  (bind _output_get (Variables|Default|SetInspectWidgetInterface _returnvalue_2))
  (UserInterface|Viewport|AddtoViewport _output_get 0)
  (Input|DisableInput _returnvalue)
  (Input|EnableInput _returnvalue))

(fn ConstructionScript)