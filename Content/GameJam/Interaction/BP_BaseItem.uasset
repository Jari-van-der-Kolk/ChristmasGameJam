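; BP_BaseItem is a configurable world item that can be inspected when the player interacts with it.
; The construction script applies the item's mesh and scale to its static mesh component.
; On interact, if Inspect is enabled, it spawns a BP_InspectItem far out along the X axis.
; It passes that actor the inspection rotation and scale, mesh, name and description, then prints a debug string.
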(event OnInteract(Interactable)
  (params (Interactor :type Interactor%20Component%20Object%20Reference) (Interactable :type Interactable%20Component%20Object%20Reference))
  (if (Variables|Public|inspection|GetInspect)
    (bind _returnvalue (Game|SpawnActorfromClass "/Game/GameJam/Interaction/BP_InspectItem.BP_InspectItem_C" (Math|Transform|MakeTransform "100000000.000000,0.000000,0.000000") "Undefined" "MultiplyWithRoot" 0 0))
    (Default|SetInspectRotation _returnvalue (Variables|Public|inspection|GetItemInspectionRotation))
    (Default|SetInspectScale _returnvalue (Variables|Public|inspection|GetItemInspectionScale))
    (Default|Inspect _returnvalue (Variables|/Script/Engine.StaticMeshComponent|GetStaticMesh (Variables|Default|GetStaticMesh)) (Variables|public|Mesh|GetItemName) (Variables|public|Mesh|GetItemDescription))
    (Development|PrintString "Hello")))

(fn ConstructionScript
  (bind _staticmesh (Variables|Default|GetStaticMesh))
  (Components|StaticMesh|SetStaticMesh (Variables|Default|GetStaticMesh) (Variables|public|Mesh|GetItemMesh))
  (Transformation|SetWorldTransform _staticmesh (Math|Transform|MakeTransform (Transformation|GetWorldLocation _staticmesh) (Transformation|GetWorldRotation _staticmesh) (Variables|public|Mesh|GetItemScale)) false false))