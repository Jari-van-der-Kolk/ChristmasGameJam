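; BP_Solver is a game jam character Blueprint that gives the player a crosshair and interaction input.
; On BeginPlay it runs parent logic, adds the crosshair widget and calls Possess on the first player controller.
; The E key forwards press and release to the Interactor component as its default key, with a leftover "Hello" debug print on press.
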(event EventBeginPlay
  (|CallParentFunction)
  (CallFunction|AddCrosshairWidget)
  (Pawn|Possess (Game|GetPlayerController 0)))

(event Input|KeyboardEvents|E
  (params (Key :type Key%20Structure :default "None"))
  (:Pressed
    (Class|InteractorComponent|InteractionInput (Variables|Default|GetInteractor) "DefaultKey" true)
    (Development|PrintString "Hello"))
  (:Released
    (Class|InteractorComponent|InteractionInput (Variables|Default|GetInteractor) "DefaultKey" false)))

(fn ConstructionScript
  (|CallParentFunction))