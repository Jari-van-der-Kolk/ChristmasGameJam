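; Main game mode that assigns joining players to the pre-placed Chaser and Solver characters, cached on BeginPlay.
; PostLogin uses a FlipFlop to alternate roles.
; The Chaser branch waits a tick, destroys the default pawn, possesses the Chaser and enables input, while the Solver branch possesses immediately.
; A helper finds both roles' PlayerStarts by tag but is not called in this graph.
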(event EventBeginPlay
  (bind _returnvalue (Actor|GetActorOfClass "/Game/GameJam/Character/CharacterTypes/BP_ChaserCharacter.BP_ChaserCharacter_C"))
  (Variables|Default|SetChaser _returnvalue)
  (bind _returnvalue_2 (Actor|GetActorOfClass "/Game/GameJam/Character/CharacterTypes/BP_SolverCharacter.BP_SolverCharacter_C"))
  (Variables|Default|SetSolver _returnvalue_2))

(event EventPostLogin
  (params (NewPlayer :type Player%20Controller%20Object%20Reference))
  (bind _chaser (Variables|Default|GetChaser))
  (Utilities|FlowControl|FlipFlop
    (:A
      (Utilities|FlowControl|DelayUntilNextTick)
      (Actor|DestroyActor (Pawn|GetControlledPawn NewPlayer))
      (Pawn|Possess NewPlayer _chaser)
      (Input|EnableInput _chaser NewPlayer))
    (:B
      (Pawn|Possess NewPlayer (Variables|Default|GetSolver)))))

(fn ConstructionScript)

(fn GetPlayerStartPositionswithTag
  (params (ChaserStartPosTag :type Name) (SolverStartPosTag :type Name))
  (bind _outactors (Actor|GetAllActorsOfClass "/Script/Engine.PlayerStart"))
  (for _array_element _outactors
    (Utilities|FlowControl|Sequence
      (:then_0
        (if (== SolverStartPosTag (Variables|/Script/Engine.PlayerStart|GetPlayerStartTag _array_element))
          (LocalVariables|SetL_SolverStart _array_element)))
      (:then_1
        (if (== (Variables|/Script/Engine.PlayerStart|GetPlayerStartTag _array_element) ChaserStartPosTag)
          (LocalVariables|SetL_ChaserStart _array_element)))))
  (return (LocalVariables|GetL_SolverStart) (LocalVariables|GetL_ChaserStart)))