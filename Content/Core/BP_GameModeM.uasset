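; BP_GameModeM is a game mode that assigns players to a Chaser or a Solver character.
; BeginPlay finds and caches one BP_ChaserCharacter and one BP_SolverCharacter already in the world.
; PostLogin counts logins: the first has player controller 0 possess the Chaser, and any later one has player controller 1 possess the Solver.
; Controllers are looked up by index rather than taken from the login event.
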(event EventBeginPlay
  (bind _returnvalue (Actor|GetActorOfClass "/Game/GameJam/Character/CharacterTypes/BP_ChaserCharacter.BP_ChaserCharacter_C"))
  (Variables|Default|SetChaser _returnvalue)
  (bind _returnvalue_2 (Actor|GetActorOfClass "/Game/GameJam/Character/CharacterTypes/BP_SolverCharacter.BP_SolverCharacter_C"))
  (Variables|Default|SetSolver _returnvalue_2))

(event EventPostLogin
  (params (NewPlayer :type Player%20Controller%20Object%20Reference))
  (bind _result (Math|Integer|IncrementInt (Variables|Default|GetLogins))
    (:%20%20
      (if (== _result 0)
        (Pawn|Possess (Game|GetPlayerController 0) (Variables|Default|GetChaser))
        (else
          (Pawn|Possess (Game|GetPlayerController 1) (Variables|Default|GetSolver)))))))

(fn ConstructionScript)